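; A door Blueprint that swings open once when the player presses E while nearby.
; Trigger overlap events set a nearby flag, and BeginPlay records the starting yaw.
; The E key plays a timeline whose track is added to that yaw to set the door's relative rotation.
; An opened flag blocks repeat activation, so the door never closes.
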(event OnComponentEndOverlap(trigger)
  (params (OtherActor :type Actor%20Object%20Reference) (OtherComp :type Primitive%20Component%20Object%20Reference) (OtherBodyIndex :type Integer))
  (Variables|DoorStatus|Setplayer-near false))

(event OnComponentBeginOverlap(trigger)
  (params (OtherActor :type Actor%20Object%20Reference) (OtherComp :type Primitive%20Component%20Object%20Reference) (OtherBodyIndex :type Integer) (bFromSweep :type Boolean) (SweepResult :type Hit%20Result%20Structure%20%28by%20ref%29))
  (Variables|DoorStatus|Setplayer-near true))

(event EventBeginPlay
  (Variables|Default|Setdoor-start (.yaw (Transformation|GetActorRotation))))

(event Input|KeyboardEvents|E
  (:Pressed
    (if (and (not (Variables|DoorStatus|Getdoor-opened)) (Variables|DoorStatus|Getplayer-near))
      (Variables|DoorStatus|Setdoor-opened true)
      (bind _door_driver_track (Timeline|Timeline%20-%20Door%20Driver Play)
        (:Update
          (Transformation|SetRelativeRotation (Class|KismetMathLibrary|MakeRot 0.0 (+ _door_driver_track (Variables|Default|Getdoor-start)) 0.0) false))))))

(fn ConstructionScript)